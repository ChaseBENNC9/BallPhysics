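; BP_Checkpoint is a one-shot checkpoint that updates the ball's respawn point on overlap.
; BeginPlay creates a dynamic M_Respawn material on the cube and paints it with the Color variable.
; The first overlap by any actor prints a message, turns it green, marks it active and plays a sound.
; Only then does it cast to BP_Ball and set SpawnLocation above itself, so a non-ball actor can consume it.
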(event `self.ReceiveBeginPlay`
  (set `self.IsActive` false)
  (bind _returnvalue (`PrimitiveComponent.CreateDynamicMaterialInstance` (`self.Cube`) 0 "/Game/StarterContent/Materials/M_Respawn.M_Respawn" "None"))
  (`MaterialInstanceDynamic.SetVectorParameterValue` _returnvalue "PaintedColor" (`KismetMathLibrary.Conv_VectorToLinearColor` (stale `ChangeColor_Event` _output_get)) :!label _label))

(event `ChangeColor_Event`
  (params (ColorValue :type "Vector Structure"))
  (bind _output_get (set `self.Color` ColorValue))
  (goto _label))

(event `self.ReceiveActorBeginOverlap`
  (params (OtherActor :type "Actor Object Reference"))
  (bind (_returnvalue_x _returnvalue_y _returnvalue_z) (`KismetMathLibrary.BreakVector` (`self.K2_GetActorLocation`)))
  (if (not (`self.IsActive`))
    (`KismetSystemLibrary.PrintText` "Checkpoint Set!")
    (`self.ChangeColor_Event` (0.0 255.0 0.0))
    (set `self.IsActive` true)
    (`GameplayStatics.PlaySoundAtLocation` "/Game/Sounds/button-confirmation_C__major.button-confirmation_C__major" (`self.K2_GetActorLocation`) (struct) 1.0 1.0 0.0 null null null null)
    (bind _asbp_ball (cast `/Game/Blueprints/BP_Ball` OtherActor))
    (set `/Game/Blueprints/BP_Ball.SpawnLocation` (`KismetMathLibrary.MakeVector` _returnvalue_x _returnvalue_y (+ _returnvalue_z 200.0)) _asbp_ball)))

(fn `UserConstructionScript`)