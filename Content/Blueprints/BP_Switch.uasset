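; BP_Switch is a one-shot overlap switch that drives a target moving platform or spinner.
; The first overlap turns its cylinder's dynamic material green, plays a confirmation sound and acts on the target by Type.
; Platforms lerp a set distance along X, Y or Z on a rate-scaled timeline, then the switch turns red.
; Spinners are simply set active through a cast to BP_Spinner.
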(event `self.ReceiveBeginPlay`
  (set `self.IsActive` false)
  (bind _returnvalue (`PrimitiveComponent.CreateDynamicMaterialInstance` (`self.Cylinder`) 0 "/Game/StarterContent/Materials/M_Respawn.M_Respawn" "None"))
  (`MaterialInstanceDynamic.SetVectorParameterValue` _returnvalue "PaintedColor" (`KismetMathLibrary.Conv_VectorToLinearColor` (stale `ChangeColor_Event` _output_get)) :!label _label))

(event `ChangeColor_Event`
  (params (ColorValue :type "Vector Structure"))
  (bind _output_get (set `self.Color` ColorValue))
  (goto _label))

(event `self.ReceiveActorBeginOverlap`
  (params (OtherActor :type "Actor Object Reference"))
  (if (not (`self.IsActive`))
    (`self.ChangeColor_Event` (0.0 255.0 0.0))
    (set `self.IsActive` true)
    (`GameplayStatics.PlaySoundAtLocation` "/Game/Sounds/button-confirmation_C__major.button-confirmation_C__major" (`self.K2_GetActorLocation`) (struct) 1.0 1.0 0.0 null null null null)
    (`self.MoveElevator_Event`)))

(event `MoveElevator_Event`
  (set `self.Start` (`self.K2_GetActorLocation` (`self.Target`)))
  (switch `/Game/LevelPrototyping/Switch_Types` (`self.Type`)
    (:`NewEnumerator0`
      (set `self.End` (+ (`self.Start`) (`KismetMathLibrary.MakeVector` (`self.TargetValue`))))
      (`TimelineComponent.SetPlayRate` (`self.Timeline`) (`self.TimeScale`) :!label _label_2)
      (bind (_direction _position) (`Timeline|Timeline` :`NewTime` 0.0 :!via `PlayFromStart`)
        (:`Update`
          ;[1 1 1] Direction X
          (`self.K2_SetActorLocation` (`self.Target`) (`KismetMathLibrary.VLerp` (`self.Start`) (`self.End`) _position) false false))
        (:`Finished`
          (set `self.Moving` (!= (`self.Moving`) true))
          (`self.ChangeColor_Event` (255.0 0.0 0.0)))))
    (:`NewEnumerator1`
      (set `self.End` (+ (`self.Start`) (`KismetMathLibrary.MakeVector` 0.0 (`self.TargetValue`))))
      (goto _label_2))
    (:`NewEnumerator2`
      (set `self.End` (+ (`self.Start`) (`KismetMathLibrary.MakeVector` 0.0 0.0 (`self.TargetValue`))))
      (goto _label_2))
    (:`NewEnumerator4`
      (bind _asbp_spinner (cast `/Game/Blueprints/BP_Spinner` (`self.Target`)))
      (set `/Game/Blueprints/BP_Spinner.IsActive` true _asbp_spinner))))

(fn `UserConstructionScript`)