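; BP_Platform is a platform actor that resets its Cube to the original placement when it hits an actor tagged "Floor".
; The construction script records the starting location and rotation, and BeginPlay teleports the actor back to that location.
; On a floor hit, very high linear and angular damping kills the Cube's motion during the teleport, then low damping returns after a short delay.
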(event `self.ReceiveBeginPlay`
  (`self.K2_SetActorLocation` (`self.SpawnLocation`) false true))

(event `self.ReceiveHit`
  (params (MyComp :type "PrimitiveComponent Object Reference") (Other :type "Actor Object Reference") (OtherComp :type "PrimitiveComponent Object Reference") (bSelfMoved :type Boolean) (HitLocation :type "Vector Structure") (HitNormal :type "Vector Structure") (NormalImpulse :type "Vector Structure") (Hit :type "HitResult Structure (by ref)"))
  (bind _cube (`self.Cube`))
  (bind _cube_2 (`self.Cube`))
  (if (`self.ActorHasTag` Other "Floor")
    (`PrimitiveComponent.SetAngularDamping` _cube 1000.0)
    (`PrimitiveComponent.SetLinearDamping` _cube 1000.0)
    (`SceneComponent.K2_SetWorldLocationAndRotation` _cube (`self.SpawnLocation`) (`self.DefaultRotation`) false true)
    (`KismetSystemLibrary.Delay` 0.2)
    (`PrimitiveComponent.SetAngularDamping` _cube_2 0.01)
    (`PrimitiveComponent.SetLinearDamping` _cube_2 0.0)))

(event `self.ReceiveActorBeginOverlap`
  (params (OtherActor :type "Actor Object Reference")))

(fn `UserConstructionScript`
  (set `self.SpawnLocation` (`self.K2_GetActorLocation`))
  (set `self.DefaultRotation` (`self.K2_GetActorRotation`)))